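; BP_CubeMatSpreader is a cube actor that spreads materials to overlapping cubes of the same class like an infection.
; Tick feeds a random Delay, so an infectious cube repeatedly picks one random overlapping spreader at irregular intervals.
; It sets that cube's material to a random MaterialToChangeTo entry and enables its CanInfect, creating a chain reaction that this graph never switches off.
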(event `self.ReceiveTick`
  (params (DeltaSeconds :type "Float (single-precision)"))
  (`KismetSystemLibrary.Delay` (`KismetMathLibrary.RandomFloatInRange` (`self.MinValue`) (`self.MaxValue`)))
  (if (`self.CanInfect`)
    (bind _asbp_cube_mat_spreader (cast `/Game/2_Blueprints/BP_CubeMatSpreader` (`KismetArrayLibrary.Array_Random` (`self.GetOverlappingActors` "BP_CubeMatSpreader_C"))))
    (`PrimitiveComponent.SetMaterial` (`/Game/2_Blueprints/BP_CubeMatSpreader.Cube` _asbp_cube_mat_spreader) 0 (`KismetArrayLibrary.Array_Random` (`self.MaterialToChangeTo`)))
    (set `/Game/2_Blueprints/BP_CubeMatSpreader.CanInfect` true _asbp_cube_mat_spreader)))

(fn `UserConstructionScript`)